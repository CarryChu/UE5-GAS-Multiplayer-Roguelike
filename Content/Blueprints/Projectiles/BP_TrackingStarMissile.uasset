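; Homing missile projectile that damages enemies through a GAS effect, with a swarm mode.
; The server starts homing on the target, after a random launch burst in swarm mode, where impact also deals area damage.
; Tick checks target health and LifeGeneration, retargeting to the living enemy nearest the instigator within range of the missile, or destroying itself.
; On hit, it multicasts a mode-specific Niagara explosion, hides and expires shortly after.
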(event OnComponentBeginOverlap(Sphere)
  (params (OverlappedComponent :type Primitive%20Component%20Object%20Reference) (OtherActor :type Actor%20Object%20Reference) (OtherComp :type Primitive%20Component%20Object%20Reference) (OtherBodyIndex :type Integer) (bFromSweep :type Boolean) (SweepResult :type Hit%20Result%20Structure%20%28by%20ref%29))
  (bind _returnvalue (Transformation|GetActorLocation))
  (bind _helix_primaryimpact (Variables|Default|GetHelix_PrimaryImpact))
  ;[0.15 0.15 0.15 0.5] 触碰到敌人后给敌人造成伤害效果
  (Networking|SwitchHasAuthority
    (:Authority
      (bind _asenemy_base (Utilities|Casting|CastToEnemyBase OtherActor))
      (if (Variables|Default|GetbIsSwarmMode)
        (CallFunction|MulticastPlayExplosion _returnvalue true)
        (bind _outactors (Collision|SphereOverlapActors _returnvalue 2e+02 (Utilities|Array|MakeArray "ObjectTypeQuery3") "/Game/Blueprints/Characters/Enemies/BP_EnemyBase.BP_EnemyBase_C"))
        (for _array_element _outactors
          (bind _asenemy_base_2 (Utilities|Casting|CastToEnemyBase _array_element))
          (GameplayEffects|ApplyGameplayEffectToTarget :self (Ability|GetAbilitySystemComponent (Variables|Actor|GetInstigator)) :GameplayEffectClass "/Game/GameplayAbilitySystem/Effects/GE_TrackingMissileDamage.GE_TrackingMissileDamage_C" :Target (Variables|/Script/MPRoguelike.EnemyBase|GetAbilitySystemComponent _asenemy_base_2)))
        (Collision|SetCollisionEnabled (Variables|Default|GetSphere) "NoCollision")
        (Development|SetHiddeninGame _helix_primaryimpact true false)
        (Components|Movement|StopMovementImmediately (Variables|Default|GetProjectileMovement))
        (Actor|SetLifeSpan 0.5)
        (else
          (GameplayEffects|ApplyGameplayEffectToTarget :self (Ability|GetAbilitySystemComponent (Variables|Actor|GetInstigator)) :GameplayEffectClass "/Game/GameplayAbilitySystem/Effects/GE_TrackingMissileDamage.GE_TrackingMissileDamage_C" :Target (Variables|/Script/MPRoguelike.EnemyBase|GetAbilitySystemComponent _asenemy_base))
          (CallFunction|MulticastPlayExplosion (Transformation|GetActorLocation) false)
          (Collision|SetCollisionEnabled (Variables|Default|GetSphere) "NoCollision")
          (Development|SetHiddeninGame _helix_primaryimpact true false)
          (Components|Movement|StopMovementImmediately (Variables|Default|GetProjectileMovement))
          (Actor|SetLifeSpan 0.5))))))

(event Custom|RetargetNewEnemy
  ;[0.15 0.15 0.15 0.5] 如果目标在导弹飞向过程中死亡后则重新搜寻最近目标
  (Variables|Default|SetMinDistance 999999.0)
  (Variables|Default|SetNewClosestEnemy 0)
  (bind _closesttarget (CallFunction|CheckTargetValidity (Variables|Default|GetPlayerAttackRange) (Transformation|GetActorLocation (Variables|Actor|GetInstigator)) (Transformation|GetActorLocation) (Utilities|Array|MakeArray "ObjectTypeQuery3")))
  (Utilities|IsValid _closesttarget
    (:Is%20Valid
      (bind _output_get (Variables|Default|SetTargetEnemy _closesttarget))
      (Variables|/Script/Engine.ProjectileMovementComponent|SetHomingTargetComponent (Variables|Default|GetProjectileMovement) (Variables|/Script/Engine.Actor|GetRootComponent _output_get)))
    (:Is%20Not%20Valid
      (Actor|DestroyActor))))

(event Custom|Multicast_PlayExplosion
  (params (ExplosionLocation :type Vector) (SwarmMode :type Boolean))
  ;[0.15 0.15 0.15 0.5] 通过多播在传入位置生成特效
  (if SwarmMode
    (Niagara|SpawnSystematLocation "/Game/Assets/VFX/Mixed_Magic_VFX_Pack/VFX/NS_Dark_Solo_Impact.NS_Dark_Solo_Impact" ExplosionLocation)
    (else
      (Niagara|SpawnSystematLocation "/Game/Assets/VFX/MixedVFX/Particles/Projectiles/Hits/NS_GalaxyArrow_Hit.NS_GalaxyArrow_Hit" ExplosionLocation))))

(event EventBeginPlay
  (bind _targetenemy (Variables|Default|GetTargetEnemy))
  (bind _projectilemovement (Variables|Default|GetProjectileMovement))
  ;[0.15 0.15 0.15 0.5] 自动追踪
  (Networking|SwitchHasAuthority
    (:Authority
      (Utilities|IsValid _targetenemy
        (:Is%20Valid
          (Variables|Default|SetLockedGeneration (Variables|/Game/Blueprints/Characters/Enemies/BP_EnemyBase.BP_EnemyBase_C|GetLifeGeneration (.AsBP%20Enemy%20Base (Utilities|Casting|CastToBP_EnemyBase _targetenemy))))
          (if (Variables|Default|GetbIsSwarmMode)
            (Game|Components|ProjectileMovement|SetVelocityinLocalSpace (Variables|Default|GetProjectileMovement) (Math|Vector|MakeVector (Math|Random|RandomFloatinRange -8e+02 8e+02) (Math|Random|RandomFloatinRange -8e+02 8e+02) (Math|Random|RandomFloatinRange 5e+02 8e+02)))
            (Utilities|FlowControl|Delay 0.2))
          (Variables|/Script/Engine.ProjectileMovementComponent|SetHomingAccelerationMagnitude _projectilemovement 3e+04)
          (Variables|/Script/Engine.MovementComponent|SetVelocity _projectilemovement "0, 0, 0")
          (Variables|/Script/Engine.ProjectileMovementComponent|SetHomingTargetComponent _projectilemovement (Variables|/Script/Engine.Actor|GetRootComponent (Variables|Default|GetTargetEnemy))))))))

(event EventTick
  (params (DeltaSeconds :type Float%20%28single-precision%29))
  (bind _targetenemy (Variables|Default|GetTargetEnemy))
  ;[0.15 0.15 0.15 0.5] 检查正在追踪的目标是否死亡，如果死亡则更换最近目标
  (Utilities|IsValid _targetenemy
    (:Is%20Valid
      (bind _asbp_enemy_base (Utilities|Casting|CastToBP_EnemyBase _targetenemy))
      (if (== (Variables|/Game/Blueprints/Characters/Enemies/BP_EnemyBase.BP_EnemyBase_C|GetLifeGeneration _asbp_enemy_base) (Variables|Default|GetLockedGeneration))
        (if (<= (.ReturnValue (Ability|Attribute|GetFloatAttributefromAbilitySystemComponent (Variables|/Script/MPRoguelike.EnemyBase|GetAbilitySystemComponent _asbp_enemy_base) "(AttributeName=\"Health\",Attribute=/Script/MPRoguelike.BasicAttributeSet:Health,AttributeOwner=\"/Script/CoreUObject.Class'/Script/MPRoguelike.BasicAttributeSet'\")")) 0.0)
          (Variables|/Script/Engine.MovementComponent|SetVelocity (Variables|Default|GetProjectileMovement) "0, 0, 0" :!label _label)
          (Utilities|FlowControl|DoOnce false :!label _label_2
            (:Completed
              (CallFunction|RetargetNewEnemy)
              (goto _label_2 Reset))))
        (else
          (goto _label))))
    (:Is%20Not%20Valid
      (goto _label))))

(fn ConstructionScript)

(fn CheckTargetValidity
  (params (SphereRadius :type Float%20%28single-precision%29) (V1 :type Vector) (SpherePos :type Vector) (ObjectTypes :type Array%20of%20EObjectTypeQuery%20Enums :default "ObjectTypeQuery1"))
  (bind _outactors (Collision|SphereOverlapActors SpherePos SphereRadius ObjectTypes "/Script/MPRoguelike.EnemyBase"))
  (for _array_element _outactors
    (bind _asbp_enemy_base (Utilities|Casting|CastToBP_EnemyBase _array_element))
    (Variables|Default|SetLockedGeneration (Variables|/Game/Blueprints/Characters/Enemies/BP_EnemyBase.BP_EnemyBase_C|GetLifeGeneration _asbp_enemy_base))
    (if (not (<= (.ReturnValue (Ability|Attribute|GetFloatAttributefromAbilitySystemComponent (Variables|/Script/MPRoguelike.EnemyBase|GetAbilitySystemComponent _asbp_enemy_base) "(AttributeName=\"Health\",Attribute=/Script/MPRoguelike.BasicAttributeSet:Health,AttributeOwner=\"/Script/CoreUObject.Class'/Script/MPRoguelike.BasicAttributeSet'\")")) 0.0))
      (if (< (Math|Vector|Distance(Vector) V1 (Transformation|GetActorLocation _array_element)) (Variables|Default|GetMinDistance))
        (Variables|Default|SetMinDistance (Math|Vector|Distance(Vector) V1 (Transformation|GetActorLocation _array_element)))
        (bind _output_get (Variables|Default|SetNewClosestEnemy _asbp_enemy_base)))))
  (return _output_get))