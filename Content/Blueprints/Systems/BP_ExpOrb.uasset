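; BP_ExpOrb is an experience pickup that flies toward a player and grants team experience when collected.
; Its outer MagnetArea sets the overlapping player as the ProjectileMovement homing target.
; Its inner PickupArea adds experience to the game state once via DoOnce, then destroys the orb.
; All logic runs on authority, and an orb with no homing target after 30 seconds destroys itself.
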(event OnComponentBeginOverlap(MagnetArea)
  (params (OverlappedComponent :type Primitive%20Component%20Object%20Reference) (OtherActor :type Actor%20Object%20Reference) (OtherComp :type Primitive%20Component%20Object%20Reference) (OtherBodyIndex :type Integer) (bFromSweep :type Boolean) (SweepResult :type Hit%20Result%20Structure%20%28by%20ref%29))
  ;[0.15 0.15 0.15 0.5] 外层：判断角色是否进入范围，进入范围后飞向玩家角色
  (Networking|SwitchHasAuthority
    (:Authority
      (bind _asbp_character_player (Utilities|Casting|CastToBP_CharacterPlayer OtherActor))
      (Variables|/Script/Engine.ProjectileMovementComponent|SetHomingTargetComponent (Variables|Default|GetProjectileMovement) (Variables|/Script/Engine.Actor|GetRootComponent _asbp_character_player)))))

(event OnComponentBeginOverlap(PickupArea)
  (params (OverlappedComponent :type Primitive%20Component%20Object%20Reference) (OtherActor :type Actor%20Object%20Reference) (OtherComp :type Primitive%20Component%20Object%20Reference) (OtherBodyIndex :type Integer) (bFromSweep :type Boolean) (SweepResult :type Hit%20Result%20Structure%20%28by%20ref%29))
  ;[0.15 0.15 0.15 0.5] 内层：触碰到玩家后自动销毁，并传递经验值
  (Networking|SwitchHasAuthority
    (:Authority
      (Utilities|Casting|CastToBP_CharacterPlayer OtherActor)
      (Utilities|FlowControl|DoOnce false
        (:Completed
          (bind _asbp_my_game_state (Utilities|Casting|CastToBP_MyGameState (Game|GetGameState)))
          (Default|AddTeamExp _asbp_my_game_state 1e+01)
          (Actor|DestroyActor))))))

(event EventBeginPlay
  ;[0.15 0.15 0.15 0.5] 如果没人拾取则30秒后自动销毁
  (Networking|SwitchHasAuthority
    (:Authority
      (Utilities|FlowControl|Delay 3e+01)
      (Utilities|IsValid (Variables|/Script/Engine.ProjectileMovementComponent|GetHomingTargetComponent (Variables|Default|GetProjectileMovement))
        (:Is%20Not%20Valid
          (Actor|DestroyActor))))))

(fn ConstructionScript)