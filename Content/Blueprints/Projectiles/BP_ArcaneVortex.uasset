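; Arcane vortex projectile that flies briefly, halts, then lives a few seconds pulling in and damaging enemies before exploding.
; A looping timer sweeps enemies in the outer sphere horizontally toward the center, scaling each step by frame delta rather than timer interval.
; A second, authority-only damage timer applies a GAS DoT effect from the Instigator to inner-sphere enemies.
; On destruction it spawns a burst system and, on authority, applies the final explosion effect within a radius.
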(event Custom|SuctionLogic
  ;[0.15 0.15 0.15 0.5] 将与Sphere重叠Enemy往Actor中间吸附
  (for _array_element (Collision|GetOverlappingActors (Variables|Default|GetSuctionSphere_Outer) "/Game/Blueprints/Characters/Enemies/BP_EnemyBase.BP_EnemyBase_C" :!class /Script/Engine.PrimitiveComponent)
    (Transformation|AddActorWorldOffset _array_element (Math|Vector|MakeVector (.X (Math|Vector|BreakVector (* (Math|Vector|Normalize (- (Transformation|GetActorLocation) (Transformation|GetActorLocation _array_element)) 1.0) (* (Utilities|Time|GetWorldDeltaSeconds) (Variables|Default|GetSuctionStrength))))) (.Y (Math|Vector|BreakVector (* (Math|Vector|Normalize (- (Transformation|GetActorLocation) (Transformation|GetActorLocation _array_element)) 1.0) (* (Utilities|Time|GetWorldDeltaSeconds) (Variables|Default|GetSuctionStrength))))) 0.0) true)))

(event Custom|DamageLogic
  ;[0.15 0.15 0.15 0.5] DamageSphere_Inner范围内每0.25S造成一次伤害
  (Networking|SwitchHasAuthority
    (:Authority
      (for _array_element (Collision|GetOverlappingActors (Variables|Default|GetDamageSphere_Inner) "/Game/Blueprints/Characters/Enemies/BP_EnemyBase.BP_EnemyBase_C" :!class /Script/Engine.PrimitiveComponent)
        (GameplayEffects|ApplyGameplayEffectToTarget :self (Ability|GetAbilitySystemComponent (Variables|Actor|GetInstigator)) :GameplayEffectClass "/Game/GameplayAbilitySystem/Effects/GE_Mage_E_DoT.GE_Mage_E_DoT_C" :Target (Ability|GetAbilitySystemComponent _array_element))))))

(event EventBeginPlay
  (Utilities|Time|SetTimerbyFunctionName 0 "SuctionLogic" 0.05 true)
  (Utilities|Time|SetTimerbyFunctionName 0 "DamageLogic" 0.25 true)
  (Utilities|FlowControl|Delay 1.0)
  (Components|Movement|StopMovementImmediately (Variables|Default|GetProjectileMovement))
  (Actor|SetLifeSpan 3.0))

(event EventDestroyed
  (Niagara|SpawnSystematLocation "/Game/Assets/VFX/Mixed_Magic_VFX_Pack/VFX/2.2" (Transformation|GetActorLocation) "0, 0, 0" "2.000000,2.000000,2.000000")
  (Networking|SwitchHasAuthority
    (:Authority
      (bind _outactors (Collision|SphereOverlapActors (Transformation|GetActorLocation) 3e+02 (Utilities|Array|MakeArray "ObjectTypeQuery3") "/Game/Blueprints/Characters/Enemies/BP_EnemyBase.BP_EnemyBase_C"))
      (for _array_element _outactors
        (GameplayEffects|ApplyGameplayEffectToTarget :self (Ability|GetAbilitySystemComponent (Variables|Actor|GetInstigator)) :GameplayEffectClass "/Game/GameplayAbilitySystem/Effects/GE_ArcaneVortex_FinalExplode.GE_ArcaneVortex_FinalExplode_C" :Target (Ability|GetAbilitySystemComponent _array_element))))))

(fn ConstructionScript)