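; BP_PlayerSlot is a lobby slot actor that displays a player's selected character.
; AddPlayer stores the player controller and reads the selected class from BP_PC_Lobby, then shares the spawn path used by SwicthCharacter.
; That path destroys any existing character, spawns the new one at the Arrow and raises it by its capsule half-height.
; RemovePlayer clears the controller and destroys the displayed character.
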(event Custom|Add%20Player
  (params (PC :type Player%20Controller%20Object%20Reference))
  (bind _arrow (Variables|Default|GetArrow))
  (bind _returnvalue (Transformation|GetWorldTransform _arrow))
  (bind _output_get (Variables|Default|SetPC PC))
  (Variables|Default|SetCharacter%20To%20Spawn (Variables|/Game/Blueprints/Lobby/BP_PC_Lobby.BP_PC_Lobby_C|GetSelected%20Character%20Class (.AsBP%20PC%20Lobby (Utilities|Casting|CastToBP_PC_Lobby _output_get))))
  (bind _selected_character (Variables|Default|GetSelected%20Character)
    (:then
      (Actor|DestroyActor _selected_character))
    (:else
      _))
  (bind _returnvalue_2 (Game|SpawnActorfromClass (Variables|Default|GetCharacter%20To%20Spawn) (Transformation|GetWorldTransform (Variables|Default|GetArrow)) "AlwaysSpawn" "MultiplyWithRoot" 0 0))
  (bind _output_get_2 (Variables|Default|SetSelected%20Character _returnvalue_2))
  (Transformation|SetActorTransform _output_get_2 (Math|Transform|MakeTransform (Math|Vector|MakeVector (.x (.location _returnvalue)) (.y (.location _returnvalue)) (+ (Components|Capsule|GetScaledCapsuleHalfHeight (Variables|/Script/Engine.Character|GetCapsuleComponent _returnvalue_2)) (.z (.location _returnvalue)))) (.rotation _returnvalue) (.scale _returnvalue))))

(event Custom|RemovePlayer
  (Variables|Default|SetPC 0)
  (bind _selected_character (Variables|Default|GetSelected%20Character)
    (:then
      (Actor|DestroyActor _selected_character)
      (Variables|Default|SetSelected%20Character 0))
    (:else)))

(event Custom|Swicth%20Character
  (params (Character%20To%20Spawn :type BP%20Third%20Person%20Character%20Class%20Reference))
  (bind _arrow (Variables|Default|GetArrow))
  (bind _returnvalue (Transformation|GetWorldTransform _arrow))
  (Variables|Default|SetCharacter%20To%20Spawn Character%20To%20Spawn)
  (bind _selected_character (Variables|Default|GetSelected%20Character)
    (:then
      (Actor|DestroyActor _selected_character))
    (:else
      _))
  (bind _returnvalue_2 (Game|SpawnActorfromClass (Variables|Default|GetCharacter%20To%20Spawn) (Transformation|GetWorldTransform (Variables|Default|GetArrow)) "AlwaysSpawn" "MultiplyWithRoot" 0 0))
  (bind _output_get (Variables|Default|SetSelected%20Character _returnvalue_2))
  (Transformation|SetActorTransform _output_get (Math|Transform|MakeTransform (Math|Vector|MakeVector (.x (.location _returnvalue)) (.y (.location _returnvalue)) (+ (Components|Capsule|GetScaledCapsuleHalfHeight (Variables|/Script/Engine.Character|GetCapsuleComponent _returnvalue_2)) (.z (.location _returnvalue)))) (.rotation _returnvalue) (.scale _returnvalue))))

(fn ConstructionScript)