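; Server-side enemy spawner that requests a pooled enemy on a looping 0.2-second timer.
; SpawnEnemy picks a point at a fixed distance and random yaw from a random player, retrying until IsLocationSafe finds no player too close.
; GetEnemyFromPool then receives a ground-plane (Z=0) location, though the random pure nodes re-roll, so it can differ from the tested point.
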(event Custom|SpawnEnemy
  ;[0.15 0.15 0.15 0.5] 对象池生成Ai敌人
  (bind _outactors (Actor|GetAllActorsOfClass "/Game/Blueprints/Characters/BP_CharacterPlayer.BP_CharacterPlayer_C" :!label _label))
  (Utilities|IsValid (.OutItem (Utilities|Array|Random _outactors))
    (:Is%20Valid
      (bind _issafe (CallFunction|IsLocationSafe (Math|Vector|MakeVector (.x (+ (Transformation|GetActorLocation (.OutItem (Utilities|Array|Random _outactors))) (* (Math|Vector|GetForwardVector (Math|Rotator|MakeRotator 0.0 0.0 (Math|Random|RandomFloatinRange 0.0 3.6e+02))) 3e+03))) (.y (+ (Transformation|GetActorLocation (.OutItem (Utilities|Array|Random _outactors))) (* (Math|Vector|GetForwardVector (Math|Rotator|MakeRotator 0.0 0.0 (Math|Random|RandomFloatinRange 0.0 3.6e+02))) 3e+03))) (.z (+ (Transformation|GetActorLocation (.OutItem (Utilities|Array|Random _outactors))) (* (Math|Vector|GetForwardVector (Math|Rotator|MakeRotator 0.0 0.0 (Math|Random|RandomFloatinRange 0.0 3.6e+02))) 3e+03))))))
      (if _issafe
        (bind _returnvalue (Class|EnemyPoolManager|GetEnemyfromPool (Math|Vector|MakeVector (.x (+ (Transformation|GetActorLocation (.OutItem (Utilities|Array|Random _outactors))) (* (Math|Vector|GetForwardVector (Math|Rotator|MakeRotator 0.0 0.0 (Math|Random|RandomFloatinRange 0.0 3.6e+02))) 3e+03))) (.y (+ (Transformation|GetActorLocation (.OutItem (Utilities|Array|Random _outactors))) (* (Math|Vector|GetForwardVector (Math|Rotator|MakeRotator 0.0 0.0 (Math|Random|RandomFloatinRange 0.0 3.6e+02))) 3e+03))) 0.0)))
        (Utilities|Casting|CastToBP_EnemyBase _returnvalue)
        (else
          (goto _label))))))

(event EventBeginPlay
  (|CallParentFunction)
  (Networking|SwitchHasAuthority
    (:Authority
      (Utilities|Time|SetTimerbyEvent (delegate Custom|SpawnEnemy) 0.2 true))))

(fn ConstructionScript)

(fn IsLocationSafe
  (params (TestLocation :type Vector))
  (bind _outactors (Actor|GetAllActorsOfClass "/Game/Blueprints/Characters/BP_CharacterPlayer.BP_CharacterPlayer_C"))
  (for _array_element _outactors
    (if (< (Math|Vector|VectorLength (- TestLocation (Transformation|GetActorLocation _array_element))) 1.5e+03)
      (return false)))
  (return true))