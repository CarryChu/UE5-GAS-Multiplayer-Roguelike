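; Game state that manages shared team experience and a synchronized level-up card-selection phase for all players.
; When experience hits a growing threshold, it raises the team level, nearly freezes global time dilation and multicasts the card screen, locking local character rotation.
; Ready calls are counted against the player array; once everyone is ready, time resumes and a multicast closes the screens, restoring game input and rotation.
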(event Custom|AddTeamExp
  (params (ExpAmount :type Float%20%28double-precision%29))
  ;[0.15 0.15 0.15 0.5] 共享经验
  (bind _output_get (Variables|Default|SetTeamExp (+ (Variables|Default|GetTeamExp) ExpAmount)))
  ;[0.15 0.15 0.15 0.5] 满经验升级后暂停游戏，并倒计时选择卡牌时间
  (if (>= _output_get (Variables|Default|GetMaxExp))
    (Variables|Default|SetTeamExp (- (Variables|Default|GetTeamExp) (Variables|Default|GetMaxExp)))
    (Variables|Default|SetMaxExp (* (Variables|Default|GetMaxExp) 1.5))
    (Variables|Default|SetTeamLevel (+ (Variables|Default|GetTeamLevel) 1))
    (Utilities|Time|SetGlobalTimeDilation 0.0001)
    (Variables|Default|SetReadyPlayersCount 0)
    (CallFunction|MulticastShowLevelUpUI)))

(event Custom|AddReadyPlayer
  ;[0.15 0.15 0.15 0.5] 判断所有玩家是否选择完卡牌
  (bind _output_get (Variables|Default|SetReadyPlayersCount (+ (Variables|Default|GetReadyPlayersCount) 1)))
  (if (>= _output_get (Utilities|Array|Length (Variables|Default|GetPlayerArray)))
    (CallFunction|FinishLevelUpPhase)))

(event Custom|Multicast_CloseLevelUpUI
  (bind _foundwidgets (Widget|GetAllWidgetsOfClass "/Game/Blueprints/UI/WBP_LevelUpScreen.WBP_LevelUpScreen_C" true))
  (for _array_element _foundwidgets
    (Input|SetInputModeUIOnly (Game|GetPlayerController 0) _array_element "DoNotLock" false)
    (Widget|RemovefromParent _array_element)
    (Input|SetInputModeGameOnly (Game|GetPlayerController 0) false)
    (Class|WidgetBlueprintLibrary|SetFocustoGameViewport)
    (bind _asbp_character_player (Utilities|Casting|CastToBP_CharacterPlayer (Game|GetPlayerCharacter 0)))
    (Variables|/Game/Blueprints/Characters/BP_CharacterPlayer.BP_CharacterPlayer_C|SetbCanRotate _asbp_character_player true)))

(event Custom|Finish_LevelUpPhase
  ;[0.15 0.15 0.15 0.5] 完成卡牌选择
  (Variables|Default|SetReadyPlayersCount 0)
  (Utilities|Time|SetGlobalTimeDilation 1.0)
  (CallFunction|MulticastCloseLevelUpUI))

(event Custom|Multicast_ShowLevelUpUI
  (if (Pawn|IsLocalPlayerController (Game|GetPlayerController 0))
    (bind _returnvalue (UserInterface|CreateWidget "/Game/Blueprints/UI/WBP_LevelUpScreen.WBP_LevelUpScreen_C"))
    (UserInterface|Viewport|AddtoViewport _returnvalue 0)
    (Default|InitCards _returnvalue)
    (Input|SetInputModeGameandUI (Game|GetPlayerController 0) 0 "DoNotLock" true false)
    (bind _asbp_character_player (Utilities|Casting|CastToBP_CharacterPlayer (Game|GetPlayerCharacter 0)))
    (Variables|/Game/Blueprints/Characters/BP_CharacterPlayer.BP_CharacterPlayer_C|SetbCanRotate _asbp_character_player false)))

(fn ConstructionScript)

(fn OnRepTeamLevel)

(fn OnRepCountdownTime)

(fn OnRepMaxExp)

(fn OnRepTeamExp)