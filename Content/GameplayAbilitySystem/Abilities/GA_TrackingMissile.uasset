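; Gameplay Ability that auto-fires tracking star missiles from the player at nearby enemies.
; Once activated, it loops through WaitDelay, stopping when the player is downed, with the upgrade card's level setting missile count and fire interval.
; Each cycle, a sphere overlap sized by an attribute picks the closest living enemy.
; If one exists, missiles spawn at random points around the player with that target, using swarm mode at higher levels.
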(event Custom|AutoFireLoop
  (bind _returnvalue (Ability|GetAvatarActorfromActorInfo))
  (bind _returnvalue_2 (Ability|GetAvatarActorfromActorInfo))
  (bind _returnvalue_3 (Transformation|GetActorLocation _returnvalue_2))
  ;[0.15 0.15 0.15 0.5] 生成自动发射导弹，并检索攻击范围内是否有敌人出现，若是没有则不生成
  (Variables|Default|SetCurrentSkillLevel (.Value (Utilities|Map|Find (Variables|/Script/MPRoguelike.UpgradeManagerComponent|GetOwnedCards (Actor|GetComponentbyClass (Ability|GetAvatarActorfromActorInfo) "/Script/MPRoguelike.UpgradeManagerComponent")) "Skill_TrackingStar-missile")))
  (bind _asbp_character_player (Utilities|Casting|CastToBP_CharacterPlayer _returnvalue_2))
  (if (not (Class|CharacterBase|GetIsDowned _asbp_character_player))
    (Variables|Default|SetMinDistance 999999.0)
    (Variables|Default|SetFoundEnemy 0)
    (bind _closesttarget (CallFunction|FindClosestEnemyWithinRange (.ReturnValue (Ability|Attribute|GetFloatAttributefromAbilitySystemComponent (Ability|GetAbilitySystemComponent _returnvalue_2) "(AttributeName=\"AttackRange\",Attribute=/Script/MPRoguelike.BasicAttributeSet:AttackRange,AttributeOwner=\"/Script/CoreUObject.Class'/Script/MPRoguelike.BasicAttributeSet'\")")) _returnvalue_3 _returnvalue_3 (Utilities|Array|MakeArray "ObjectTypeQuery3")))
    (Utilities|IsValid _closesttarget
      (:Is%20Valid
        (for _index (range 1 (Utilities|Select :Index (Variables|Default|GetCurrentSkillLevel) :Option%200 0 :Option%201 1 :Option%202 2 :Option%203 2 :Option%204 4 :Option%205 8))
          (Game|SpawnActorfromClass "/Game/Blueprints/Projectiles/BP_TrackingStarMissile.BP_TrackingStarMissile_C" (Math|Transform|MakeTransform (Math|Random|RandomPointinBoundingBox (Transformation|GetActorLocation (Ability|GetAvatarActorfromActorInfo)) "50.000000,50.000000,50.000000")) "AlwaysSpawn" "MultiplyWithRoot" (Components|GetOwner _returnvalue) (Variables|Default|GetFoundEnemy) (.ReturnValue (Ability|Attribute|GetFloatAttributefromAbilitySystemComponent (Ability|GetAbilitySystemComponent _returnvalue) "(AttributeName=\"AttackRange\",Attribute=/Script/MPRoguelike.BasicAttributeSet:AttackRange,AttributeOwner=\"/Script/CoreUObject.Class'/Script/MPRoguelike.BasicAttributeSet'\")")) (>= (Variables|Default|GetCurrentSkillLevel) 4) (Variables|/Script/Engine.Actor|GetInstigator _returnvalue))))
      (:Is%20Not%20Valid
        _))
    (Ability|Tasks|WaitDelay (Utilities|Select :Index (Variables|Default|GetCurrentSkillLevel) :Option%200 1.5 :Option%201 1.5 :Option%202 1.2 :Option%203 0.8 :Option%204 0.8 :Option%205 0.5)
      (:OnFinish
        (CallFunction|AutoFireLoop)))))

(event Ability|EventActivateAbility
  (Ability|CommitAbility)
  (CallFunction|AutoFireLoop))

(fn FindClosestEnemyWithinRange
  (params (SphereRadius :type Float%20%28single-precision%29) (InputPin :type Vector) (SpherePos :type Vector) (ObjectTypes :type Array%20of%20EObjectTypeQuery%20Enums :default "ObjectTypeQuery1"))
  (bind _outactors (Collision|SphereOverlapActors SpherePos SphereRadius ObjectTypes "/Game/Blueprints/Characters/Enemies/BP_EnemyBase.BP_EnemyBase_C"))
  (for _array_element _outactors
    (bind _asbp_enemy_base (Utilities|Casting|CastToBP_EnemyBase _array_element))
    (if (not (<= (.ReturnValue (Ability|Attribute|GetFloatAttributefromAbilitySystemComponent (Variables|/Script/MPRoguelike.EnemyBase|GetAbilitySystemComponent _asbp_enemy_base) "(AttributeName=\"Health\",Attribute=/Script/MPRoguelike.BasicAttributeSet:Health,AttributeOwner=\"/Script/CoreUObject.Class'/Script/MPRoguelike.BasicAttributeSet'\")")) 0.0))
      (if (< (Math|Vector|Distance(Vector) (Transformation|GetActorLocation _array_element) InputPin) (Variables|Default|GetMinDistance))
        (Variables|Default|SetMinDistance (Math|Vector|Distance(Vector) (Transformation|GetActorLocation _array_element) InputPin))
        (bind _output_get (Variables|Default|SetFoundEnemy _asbp_enemy_base)))))
  (return _output_get))