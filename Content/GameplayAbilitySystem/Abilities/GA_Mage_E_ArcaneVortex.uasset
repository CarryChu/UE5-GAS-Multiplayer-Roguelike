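; GA_Mage_E_ArcaneVortex is the Mage's E-skill gameplay ability that casts an Arcane Vortex.
; On activation it commits, then listens for the Event.Mage.SpawnVortex gameplay event while playing the AM_Mage_ESkill montage.
; When the event arrives, it spawns BP_ArcaneVortex a short distance in front of the avatar, facing the same way.
; The ability ends when the montage completes, blends out, is interrupted or is cancelled.
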(event Ability|EventActivateAbility
  (bind _returnvalue (Ability|GetAvatarActorfromActorInfo))
  (Ability|CommitAbility)
  (Utilities|FlowControl|Sequence
    (:then_0
      (Ability|Tasks|WaitGameplayEvent "(TagName=\"Event.Mage.SpawnVortex\")" 0
        (:EventReceived
          (Game|SpawnActorfromClass "/Game/Blueprints/Projectiles/BP_ArcaneVortex.BP_ArcaneVortex_C" (Math|Transform|MakeTransform (+ (Transformation|GetActorLocation _returnvalue) (* (Transformation|GetActorForwardVector _returnvalue) 1.5e+02)) (Transformation|GetActorRotation _returnvalue) "1.000000,1.000000,1.000000") "AlwaysSpawn" "MultiplyWithRoot" 0 (Variables|/Script/Engine.Actor|GetInstigator (Ability|GetAvatarActorfromActorInfo))))))
    (:then_1
      (|PlayMontageandWaitProxy "None" "/Game/Blueprints/Characters/Player/Anims/AM_Mage_ESkill.AM_Mage_ESkill" 1.0 "None" true 1.0 0.0 false
        (:OnCompleted
          _)
        (:OnBlendOut
          _)
        (:OnInterrupted
          _)
        (:OnCancelled
          _))
      (Ability|EndAbility))))