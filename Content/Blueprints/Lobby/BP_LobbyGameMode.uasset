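; Lobby game mode that seats joining players in BP_PlayerSlot actors, tracks character choice and readiness, and starts the match.
; Slots are ordered by index tag on BeginPlay; login and logout reconcile them with the controller list after a delay-loop macro confirms setup.
; Player info updates refresh slot characters, save selections in BP_GameInstance and set all-ready on the first controller's UI.
; StartMatch server-travels to GameMap and notifies each controller.
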(event EventBeginPlay
  (CallFunction|SetPlayerSlots))

(event EventPostLogin
  (params (NewPlayer :type Player%20Controller%20Object%20Reference))
  (Utilities|Array|Add (Variables|Default|GetPCs) NewPlayer)
  (Utilities|IfPlayerSlotsSet
    (:真
      (CallFunction|UpdataPlayerSlots))))

(event EventOnLogout
  (params (ExitingController :type Controller%20Object%20Reference))
  (bind _as玩家控制器 (Utilities|Casting|CastToPlayerController ExitingController))
  (Utilities|Array|RemoveItem (Variables|Default|GetPCs) _as玩家控制器)
  (Utilities|IfPlayerSlotsSet
    (:真
      (CallFunction|UpdataPlayerSlots))))

(fn ConstructionScript)

(fn SetPlayerSlots
  (bind _outactors (Actor|GetAllActorsOfClass "/Game/Blueprints/Lobby/BP_PlayerSlot.BP_PlayerSlot_C"))
  (for _index (range 0 (Utilities|Array|LastIndex _outactors))
    (bind _outactors_2 (Actor|GetAllActorsOfClasswithTag "/Game/Blueprints/Lobby/BP_PlayerSlot.BP_PlayerSlot_C" (Utilities|String|StringToName (Utilities|String|ToString(Integer) _index))))
    (Utilities|Array|Add (Variables|Default|GetPlayer%20Slots) (Utilities|Array|Get(acopy) _outactors_2)))
  (Variables|Default|SetSetSlotsDone? true))

(fn UpdataPlayerSlots
  ;[0.15 0.15 0.15 0.5] 检查
  (for _array_element (Variables|Default|GetPCs)
    (LocalVariables|SetPC%20Already%20Added? false)
    (bind _array_element_2 (Utilities|Array|ForEachLoopwithBreak (Variables|Default|GetPlayer%20Slots) :!label _label)
      (:LoopBody
        (if (== (Variables|/Game/Blueprints/Lobby/BP_PlayerSlot.BP_PlayerSlot_C|GetPC _array_element_2) _array_element)
          (LocalVariables|SetPC%20Already%20Added? true)
          (goto _label Break)))
      (:Completed
        ;[0.15 0.15 0.15 0.5] Add PC to Player
        (if (not (LocalVariables|GetPC%20Already%20Added?))
          (bind _array_element_3 (Utilities|Array|ForEachLoopwithBreak (Variables|Default|GetPlayer%20Slots) :!label _label_2)
            (:LoopBody
              (Variables|/Game/Blueprints/Lobby/BP_PlayerSlot.BP_PlayerSlot_C|GetPC _array_element_3
                (:then)
                (:else
                  (Default|AddPlayer _array_element_3 _array_element)
                  (goto _label_2 Break)))))))))
  ;[0.15 0.15 0.15 0.5] Remove断开玩家插槽连接
  (for _array_element_4 (Variables|Default|GetPlayer%20Slots)
    (if (not (Utilities|Array|ContainsItem (Variables|Default|GetPCs) (Variables|/Game/Blueprints/Lobby/BP_PlayerSlot.BP_PlayerSlot_C|GetPC _array_element_4)))
      (Default|RemovePlayer _array_element_4))))

(fn UpdataPlayerInfo
  (params (Requesting%20PC :type Player%20Controller%20Object%20Reference))
  (bind _asbp_pc_lobby (Utilities|Casting|CastToBP_PC_Lobby Requesting%20PC))
  (bind _asbp_pc_lobby_2 (Utilities|Casting|CastToBP_PC_Lobby Requesting%20PC))
  (bind _selected_character_class (Variables|/Game/Blueprints/Lobby/BP_PC_Lobby.BP_PC_Lobby_C|GetSelected%20Character%20Class _asbp_pc_lobby_2))
  (bind _array_element (Utilities|Array|ForEachLoopwithBreak (Variables|Default|GetPlayer%20Slots))
    (:LoopBody
      (if (== (Variables|/Game/Blueprints/Lobby/BP_PlayerSlot.BP_PlayerSlot_C|GetPC _array_element) Requesting%20PC)
        (if (== (Utilities|GetClass (Variables|/Game/Blueprints/Lobby/BP_PlayerSlot.BP_PlayerSlot_C|GetSelected%20Character _array_element)) _selected_character_class)
          _
          (else
            (Default|SwicthCharacter _array_element _selected_character_class)))
        (Default|UpdataPlayerInfo (.AsBP%20Character%20Player (Utilities|Casting|CastToBP_CharacterPlayer (Variables|/Game/Blueprints/Lobby/BP_PlayerSlot.BP_PlayerSlot_C|GetSelected%20Character _array_element))) (Utilities|Struct|MakeS_PlayerInfo Requesting%20PC (Utilities|Text|ToText(String) (Class|AdvancedSessionsLibrary|GetPlayerName Requesting%20PC)) (.ready? (Variables|/Game/Blueprints/Lobby/BP_PC_Lobby.BP_PC_Lobby_C|GetPlayer%20Info (.AsBP%20PC%20Lobby (Utilities|Casting|CastToBP_PC_Lobby Requesting%20PC)))) (Variables|/Script/Engine.Controller|GetPlayerState Requesting%20PC)))
        (CallFunction|CheckAllPlayerReady?)
        (Utilities|Map|Add (Variables|/Game/Blueprints/BP_GameInstance.BP_GameInstance_C|GetSelectedCharacterOfAll (.AsBP%20Game%20Instance (Utilities|Casting|CastToBP_GameInstance (Game|GetGameInstance)))) (Class|AdvancedSessionsLibrary|GetPlayerName _asbp_pc_lobby) (Variables|/Game/Blueprints/Lobby/BP_PC_Lobby.BP_PC_Lobby_C|GetSelected%20Character%20Class _asbp_pc_lobby))
        (return)))
    (:Completed
      (Default|UpdataPlayerInfo (.AsBP%20PC%20Lobby (Utilities|Casting|CastToBP_PC_Lobby Requesting%20PC))))))

(fn CheckAllPlayerReady?
  (LocalVariables|SetAll%20Player%20Ready? true)
  (for _array_element (Variables|Default|GetPCs)
    (if (not (.ready? (Variables|/Game/Blueprints/Lobby/BP_PC_Lobby.BP_PC_Lobby_C|GetPlayer%20Info (.AsBP%20PC%20Lobby (Utilities|Casting|CastToBP_PC_Lobby _array_element)))))
      (LocalVariables|SetAll%20Player%20Ready? false)))
  (Variables|/Game/Blueprints/UI/WBP_LobbyUI.WBP_LobbyUI_C|SetAll%20Player%20Ready? (Variables|/Game/Blueprints/Lobby/BP_PC_Lobby.BP_PC_Lobby_C|GetLobby%20UI (.AsBP%20PC%20Lobby (Utilities|Casting|CastToBP_PC_Lobby (Game|GetPlayerController 0)))) (LocalVariables|GetAll%20Player%20Ready?)))

(fn StartMatch
  (Class|AdvancedSessionsLibrary|ServerTravel "GameMap" false false)
  (for _array_element (Variables|Default|GetPCs)
    (bind _asbp_pc_lobby (Utilities|Casting|CastToBP_PC_Lobby _array_element))
    (Default|OnStartMatch _asbp_pc_lobby)))