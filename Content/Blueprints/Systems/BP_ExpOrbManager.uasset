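; BP_ExpOrbManager renders experience orbs and passes picked-up experience to the team total.
; Every Tick it clears one Instanced Static Mesh component and rebuilds an instance at each location in OrbList, so orbs are data entries.
; OnOrbPickedUp casts the game state to BP_MyGameState and calls AddTeamExp with the amount.
; This graph neither fills OrbList nor detects pickups.
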(event EventBeginPlay)

(event Collision|EventActorBeginOverlap
  (params (OtherActor :type Actor%20Object%20Reference)))

(event EventTick
  (params (DeltaSeconds :type Float%20%28single-precision%29))
  (Components|InstancedStaticMesh|ClearInstances (Variables|Default|GetInstancedStaticMesh))
  (for _array_element (Variables|Default|GetOrbList)
    (Components|InstancedStaticMesh|AddInstance (Variables|Default|GetInstancedStaticMesh) (Math|Transform|MakeTransform (.Location (Utilities|Struct|BreakExpOrbData _array_element)) "0, 0, 0" "1.000000,1.000000,1.000000") false)))

(event EventOnOrbPickedUp
  (params (ExpAmount :type Float%20%28single-precision%29) (Picker :type Actor%20Object%20Reference))
  (bind _asbp_my_game_state (Utilities|Casting|CastToBP_MyGameState (Game|GetGameState)))
  (Default|AddTeamExp _asbp_my_game_state ExpAmount))

(fn ConstructionScript)