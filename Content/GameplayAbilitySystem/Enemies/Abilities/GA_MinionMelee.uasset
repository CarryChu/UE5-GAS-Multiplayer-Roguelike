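; GA_MinionMelee is a gameplay ability that performs a minion's melee attack on its target player.
; On activation it commits, plays the attack montage and waits for the AttackHit gameplay event.
; When that event arrives, it applies GE_MinionDamage only if the enemy's TargetPlayer is valid and within a fixed melee range.
; The ability ends when the montage completes, is interrupted or is cancelled.
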(event Ability|EventActivateAbility
  (bind _returnvalue (Ability|GetAvatarActorfromActorInfo))
  (Ability|CommitAbility)
  (Utilities|FlowControl|Sequence
    (:then_0
      (Ability|Tasks|WaitGameplayEvent "(TagName=\"Event.Minion.AttackHit\")" 0
        (:EventReceived
          (bind _asbp_enemy_base (Utilities|Casting|CastToBP_EnemyBase _returnvalue))
          (Utilities|IsValid (Variables|/Game/Blueprints/Characters/Enemies/BP_EnemyBase.BP_EnemyBase_C|GetTargetPlayer _asbp_enemy_base)
            (:Is%20Valid
              (if (<= (Math|Vector|Distance(Vector) (Transformation|GetActorLocation _returnvalue) (Transformation|GetActorLocation (Variables|/Game/Blueprints/Characters/Enemies/BP_EnemyBase.BP_EnemyBase_C|GetTargetPlayer _asbp_enemy_base))) 1.8e+02)
                (GameplayEffects|ApplyGameplayEffectToTarget :self (Ability|GetAbilitySystemComponent _returnvalue) :GameplayEffectClass "/Game/GameplayAbilitySystem/Enemies/Effects/GE_MinionDamage.GE_MinionDamage_C" :Target (Ability|GetAbilitySystemComponent (Variables|/Game/Blueprints/Characters/Enemies/BP_EnemyBase.BP_EnemyBase_C|GetTargetPlayer _asbp_enemy_base)))))))))
    (:then_1
      (|PlayMontageandWaitProxy "None" "/Game/Blueprints/Characters/Enemies/Anims/AM_MinionAttack.AM_MinionAttack" 1.0 "None" true 1.0 0.0 false
        (:OnCompleted
          _)
        (:OnInterrupted
          _)
        (:OnCancelled
          _))
      (Ability|EndAbility))))

(event Ability|EventOnEndAbility
  (params (bWasCancelled :type Boolean)))