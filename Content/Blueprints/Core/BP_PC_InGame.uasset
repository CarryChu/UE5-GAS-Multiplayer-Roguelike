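; In-game player controller that sets up local input and HUD and relays level-up phase events to the game state.
; On BeginPlay, the local controller adds the default input mapping, shows the game timer widget and pre-spawns a pool of damage actors to avoid repeated creation.
; Server_SelectCard registers a ready player without using the card ID, while Server_TimeIsUp ends the level-up phase, both through BP_MyGameState.
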(event Custom|Server_SelectCard
  (params (CardID :type Integer))
  (bind _asbp_my_game_state (Utilities|Casting|CastToBP_MyGameState (Game|GetGameState)))
  (Default|AddReadyPlayer _asbp_my_game_state))

(event Custom|Server_TimeIsUp
  (bind _asbp_my_game_state (Utilities|Casting|CastToBP_MyGameState (Game|GetGameState)))
  (Default|FinishLevelUpPhase _asbp_my_game_state))

(event EventBeginPlay
  (bind _returnvalue (PlayerController|LocalPlayerSubsystems|GetEnhancedInputLocalPlayerSubsystem))
  (if (Pawn|IsLocalPlayerController)
    (Input|SetInputModeGameandUI self 0 "DoNotLock" false false)
    (Utilities|IsValid _returnvalue
      (:Is%20Valid
        (Input|AddMappingContext _returnvalue "/Game/Assets/Input/IMC_Default.IMC_Default" 0 "(bIgnoreAllPressedKeysUntilRelease=True,bForceImmediately=False,bNotifyUserSettings=False)")
        ;[0.15 0.15 0.15 0.5] 初始生成受伤UI，防止以后每次攻击Enemy时都要生成一个新的UI和进行销毁而浪费内存
        (bind _returnvalue_2 (UserInterface|CreateWidget "/Game/Blueprints/UI/WBP_GameTimer.WBP_GameTimer_C"))
        (UserInterface|Viewport|AddtoViewport _returnvalue_2 0)
        (for _index (range 0 150)
          (bind _returnvalue_3 (Game|SpawnActorfromClass "/Game/Blueprints/Characters/Enemies/BP_DamageActor.BP_DamageActor_C" (Math|Transform|MakeTransform "0, 0, 0" "0, 0, 0" "1.000000,1.000000,1.000000") "Undefined" "MultiplyWithRoot" 0 0.0 0))
          (Utilities|Array|Add (Variables|Default|GetDamageTextPool) _returnvalue_3))))))

(event EventTick
  (params (DeltaSeconds :type Float%20%28single-precision%29)))

(fn ConstructionScript)