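; GA_Fireball is a Gameplay Ability that launches the mage's fireball.
; On activation it commits, spawns BP_Fireball at the BP_Mage avatar's Muzzle transform, then ends immediately.
; The spawn passes in a lifespan computed from an avatar attribute divided by a fixed constant, plus an outgoing GE_FireballDamage spec handle, so the projectile carries its own damage effect.
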(event Ability|EventActivateAbility
  (bind _returnvalue (Ability|GetAvatarActorfromActorInfo))
  ;[0.15 0.15 0.15 0.5] 法球生成
  (Ability|CommitAbility)
  (Game|SpawnActorfromClass "/Game/Blueprints/Projectiles/BP_Fireball.BP_Fireball_C" (Transformation|GetWorldTransform (Variables|/Game/Blueprints/Characters/Player/BP_Mage.BP_Mage_C|GetMuzzle (.AsBP%20Mage (Utilities|Casting|CastToBP_Mage _returnvalue)))) "Undefined" "MultiplyWithRoot" 0 (/ (.ReturnValue (Ability|Attribute|GetFloatAttributefromAbilitySystemComponent (Ability|GetAbilitySystemComponent _returnvalue) "(AttributeName=\"AttackRange\",Attribute=/Script/MPRoguelike.BasicAttributeSet:AttackRange,AttributeOwner=\"/Script/CoreUObject.Class'/Script/MPRoguelike.BasicAttributeSet'\")")) 1.5e+03) (GameplayEffects|MakeOutgoingSpec :self (Ability|GetAbilitySystemComponent _returnvalue) :GameplayEffectClass "/Game/GameplayAbilitySystem/Effects/GE_FireballDamage.GE_FireballDamage_C") 0)
  (Ability|EndAbility))

(event Ability|EventOnEndAbility
  (params (bWasCancelled :type Boolean)))