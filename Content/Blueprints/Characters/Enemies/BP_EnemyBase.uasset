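; Base pooled enemy character using the Gameplay Ability System.
; On the server it turns toward its target player within range, activates its attack ability, and damages players on overlap.
; Health changes drive the overhead bar, pooled damage numbers and death, which spawns experience, counts the kill and sleeps the enemy.
; WakeUp resets stats through a SetByCaller effect; hit reactions add knockback, brief time-dilation hit-stop, flash and sound.
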(event OnComponentBeginOverlap(CapsuleComponent)
  (params (OverlappedComponent :type Primitive%20Component%20Object%20Reference) (OtherActor :type Actor%20Object%20Reference) (OtherComp :type Primitive%20Component%20Object%20Reference) (OtherBodyIndex :type Integer) (bFromSweep :type Boolean) (SweepResult :type Hit%20Result%20Structure%20%28by%20ref%29))
  ;[0.15 0.15 0.15 0.5] 触碰玩家扣血
  (Networking|SwitchHasAuthority
    (:Authority
      (bind _asbp_character_player (Utilities|Casting|CastToBP_CharacterPlayer OtherActor))
      (GameplayEffects|ApplyGameplayEffectToSelf :self (Variables|/Script/MPRoguelike.CharacterBase|GetAbilitySystemComponent _asbp_character_player) :GameplayEffectClass "/Game/GameplayAbilitySystem/Enemies/Effects/GE_MonsterDamage.GE_MonsterDamage_C"))))

(event Custom|CheckDeath
  ;[0.15 0.15 0.15 0.5] 怪物死亡逻辑
  (if (<= (.ReturnValue (Ability|Attribute|GetFloatAttributefromAbilitySystemComponent (Variables|Default|GetAbilitySystemComponent) "(AttributeName=\"Health\",Attribute=/Script/MPRoguelike.BasicAttributeSet:Health,AttributeOwner=\"/Script/CoreUObject.Class'/Script/MPRoguelike.BasicAttributeSet'\")")) 0.0)
    (Utilities|FlowControl|Delay 0.1)
    (CallFunction|MulticastSetEnemyVisualState false)
    (if (not (Variables|Default|GetbIsSleeping))
      (Networking|SwitchHasAuthority
        (:Authority
          (bind _returnvalue (Actor|GetActorOfClass "/Game/Blueprints/Systems/BP_ExpOrbManager.BP_ExpOrbManager_C"))
          (Class|ExpOrbManager|AddExpOrb _returnvalue (.location (Transformation|GetActorTransform)) 4e+01)
          (bind _asbp_my_game_state (Utilities|Casting|CastToBP_MyGameState (Game|GetGameState)))
          (Variables|/Game/Blueprints/Core/BP_MyGameState.BP_MyGameState_C|SetTotalKillCount _asbp_my_game_state (+ (Variables|/Game/Blueprints/Core/BP_MyGameState.BP_MyGameState_C|GetTotalKillCount _asbp_my_game_state) 1))
          (Class|EnemyBase|GotoSleep))))))

(event Custom|Multicast_SetEnemyVisualState
  (params (bIsVisible :type Boolean))
  (Rendering|SetVisibility (Variables|Default|GetHealthBarWidget) bIsVisible false)
  (Collision|SetActorEnableCollision bIsVisible))

(event Custom|UpdateHealthUI
  (params (OldHealth :type Float%20%28double-precision%29) (NewHealth :type Float%20%28double-precision%29))
  (bind _returnvalue (- OldHealth NewHealth))
  ;[0.15 0.15 0.15 0.5] 更新Ai血量
  (if (> (.Z (Math|Vector|BreakVector (Transformation|GetActorLocation))) -5e+02)
    (bind _aswbp_overhead_health (Utilities|Casting|CastToWBP_OverheadHealth (UserInterface|GetUserWidgetObject (Variables|Default|GetHealthBarWidget))))
    (Variables|/Game/Blueprints/UI/WBP_OverheadHealth.WBP_OverheadHealth_C|SetCurrentHealthPercent _aswbp_overhead_health (/ NewHealth (.ReturnValue (Ability|Attribute|GetFloatAttributefromAbilitySystemComponent (Variables|Default|GetAbilitySystemComponent) "(AttributeName=\"MaxHealth\",Attribute=/Script/MPRoguelike.BasicAttributeSet:MaxHealth,AttributeOwner=\"/Script/CoreUObject.Class'/Script/MPRoguelike.BasicAttributeSet'\")"))))
    (if (> _returnvalue 0.0)
      (bind _asbp_pc_in_game (Utilities|Casting|CastToBP_PC_InGame (Game|GetPlayerController 0)))
      (bind _array_element (Utilities|Array|ForEachLoopwithBreak (Variables|/Game/Blueprints/Core/BP_PC_InGame.BP_PC_InGame_C|GetDamageTextPool _asbp_pc_in_game) :!label _label)
        (:LoopBody
          (if (Variables|/Script/Engine.Actor|GetbHidden _array_element)
            (Default|WakeUpDamage _array_element _returnvalue (+ (Transformation|GetActorLocation) "0.000000,0.000000,80.000000"))
            (goto _label Break)))
        (:Completed
          (CallFunction|CheckDeath :!label _label_2)))
      (else
        (goto _label_2)))))

(event Custom|HaltAILogic
  (bind _asai控制器 (Utilities|Casting|CastToAIController (Pawn|GetController)))
  (AI|Navigation|StopMovement _asai控制器)
  (Pawn|Components|CharacterMovement|DisableMovement (Variables|Character|GetCharacterMovement)))

(event EventOnHealthChanged
  (params (OldValue :type Float%20%28single-precision%29) (NewValue :type Float%20%28single-precision%29))
  (CallFunction|UpdateHealthUI OldValue NewValue))

(event EventOnClientWakeUpUI
  (Utilities|FlowControl|Delay 0.2)
  (CallFunction|UpdateHealthUI 0.0 (Variables|Default|GetInitialHealth)))

(event EventTick
  (params (DeltaSeconds :type Float%20%28single-precision%29))
  (bind _returnvalue (Transformation|GetActorLocation))
  (bind _targetplayer (Variables|Default|GetTargetPlayer))
  (bind _targetplayer_2 (Variables|Default|GetTargetPlayer))
  (bind _returnvalue_2 (Transformation|GetActorLocation _targetplayer_2))
  (bind _returnvalue_3 (Math|Rotator|FindLookatRotation _returnvalue _returnvalue_2))
  (Networking|SwitchHasAuthority
    (:Authority
      ;[0.15 0.15 0.15 0.5] 计算与玩家角色的距离
      (Utilities|IsValid _targetplayer
        (:Is%20Valid
          (if (not (> (Transformation|GetDistanceTo self _targetplayer) (Variables|Default|GetInitAttackRange)))
            ;[0.15 0.15 0.15 0.5] 判断是否朝向玩家
            (if (not (GameplayTags|HasMatchingGameplayTag (Variables|Default|GetAbilitySystemComponent) "(TagName=\"State.Attacking\")"))
              (if (< (Math|Float|Absolute(Float) (.yaw (Math|Rotator|Delta(Rotator) (Transformation|GetActorRotation) _returnvalue_3))) 15.0)
                ;[0.15 0.15 0.15 0.5] 距离内自动攻击
                (Transformation|SetActorRotation (Math|Rotator|MakeRotator 0.0 0.0 (.yaw (Math|Rotator|FindLookatRotation (Transformation|GetActorLocation) (Transformation|GetActorLocation (Variables|Default|GetTargetPlayer))))))
                (Abilities|TryActivateAbilitybyClass (Variables|Default|GetAbilitySystemComponent) (Variables|Default|GetDefaultAttackAbility) true)
                (else
                  ;[0.15 0.15 0.15 0.5] 朝向玩家
                  (Transformation|SetActorRotation (Math|Interpolation|RInterpTo (Transformation|GetActorRotation) _returnvalue_3 (Utilities|Time|GetWorldDeltaSeconds) 5.0)))))))))))

(event EventWakeUp
  (params (Location :type Vector :default "0, 0, 0"))
  ;[0.15 0.15 0.15 0.5] 重置NPC对象池血量状态等
  (|CallParentFunction Location)
  (bind _returnvalue (Ability|GameplayEffect|AssignTagSetbyCallerMagnitude (GameplayEffects|MakeOutgoingSpec :self (Variables|Default|GetAbilitySystemComponent) :GameplayEffectClass "/Game/GameplayAbilitySystem/Enemies/Effects/GE_ResetStats.GE_ResetStats_C" :Level 1.0) "(TagName=\"Data.MaxHealth.ResetValue\")" (Variables|Default|GetInitialMaxHealth)))
  (bind _returnvalue_2 (Ability|GameplayEffect|AssignTagSetbyCallerMagnitude _returnvalue "(TagName=\"Data.Health.ResetValue\")" (Variables|Default|GetInitialHealth)))
  (bind _returnvalue_3 (Ability|GameplayEffect|AssignTagSetbyCallerMagnitude _returnvalue_2 "(TagName=\"Data.MovementSpeed.ResetValue\")" (Variables|Default|GetInitialMoveSpeed)))
  (bind _returnvalue_4 (Ability|GameplayEffect|AssignTagSetbyCallerMagnitude _returnvalue_3 "(TagName=\"Data.AttackSpeed.ResetValue\")" (Variables|Default|GetInitialAttackSpeed)))
  (bind _returnvalue_5 (Ability|GameplayEffect|AssignTagSetbyCallerMagnitude _returnvalue_4 "(TagName=\"Data.AttackPower.ResetValue\")" (Variables|Default|GetInitialAttackPower)))
  (bind _returnvalue_6 (Ability|GameplayEffect|AssignTagSetbyCallerMagnitude _returnvalue_5 "(TagName=\"Data.AttackRange.ResetValue\")" (Variables|Default|GetInitAttackRange)))
  (GameplayEffects|ApplyGameplayEffectSpecToSelf (Variables|Default|GetAbilitySystemComponent) _returnvalue_6)
  (Rendering|Material|SetOverlayMaterial (Variables|Character|GetMesh) 0 :!class /Script/Engine.MeshComponent))

(event EventBeginPlay
  (|CallParentFunction)
  (Networking|SwitchHasAuthority
    (:Authority
      (GameplayAbilities|GiveAbility (Variables|Default|GetAbilitySystemComponent) (Variables|Default|GetDefaultAttackAbility) 0 -1)
      (CallFunction|UpdateHealthUI 0.0 (Variables|Default|GetInitialHealth)))))

(event EventOnTakeHitReact
  (params (DamageCauser :type Actor%20Object%20Reference))
  (bind _mesh (Variables|Character|GetMesh))
  ;[0.15 0.15 0.15 0.5] 被击打后卡顿打击感效果，模型闪白
  (Utilities|IsValid DamageCauser
    (:Is%20Valid
      (Utilities|FlowControl|Sequence
        (:then_0
          (Character|LaunchCharacter (+ (* (Math|Vector|Normalize (- (Transformation|GetActorLocation) (Transformation|GetActorLocation DamageCauser))) 1e+02) (Math|Vector|MakeVector 0.0 0.0 0.0)) true true))
        (:then_1
          (Variables|Default|SetCustomTimeDilation 0.1)
          (Utilities|FlowControl|Delay 0.005)
          (Variables|Default|SetCustomTimeDilation 1.0)
          (Rendering|Material|SetOverlayMaterial _mesh "/Game/Blueprints/UI/Material/M_HitFlash.M_HitFlash" :!class /Script/Engine.MeshComponent)
          (Utilities|FlowControl|RetriggerableDelay 0.2)
          (Rendering|Material|SetOverlayMaterial _mesh 0 :!class /Script/Engine.MeshComponent))
        (:then_2
          (Audio|PlaySoundatLocation "/Game/Assets/Audio/universfield-thud-291047.universfield-thud-291047" (Transformation|GetActorLocation) "0, 0, 0" 2.0 (Math|Random|RandomFloatinRange 0.85 1.15) 0.15 "/Game/Assets/Audio/SA_Magic.SA_Magic" "/Game/Assets/Audio/SC_Hit.SC_Hit" 0 0))))))

(fn ConstructionScript)