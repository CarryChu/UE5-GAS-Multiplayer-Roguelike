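; Gameplay ability for an enemy ranged attack that fires a projectile at the enemy's target player.
; On activation it commits, plays the ranged attack montage and listens for the AttackHit gameplay event.
; The event spawns an enemy projectile at the front muzzle socket, rotated toward the target and carrying a minion damage effect spec.
; The ability ends when the montage completes, is interrupted or is cancelled.
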(event Ability|EventActivateAbility
  (Ability|CommitAbility)
  (Utilities|FlowControl|Sequence
    (:then_0
      (Ability|Tasks|WaitGameplayEvent "(TagName=\"Event.Minion.AttackHit\")" 0
        (:EventReceived
          (bind _asbp_enemy_base (Utilities|Casting|CastToBP_EnemyBase (Ability|GetAvatarActorfromActorInfo)))
          (Utilities|IsValid (Variables|/Game/Blueprints/Characters/Enemies/BP_EnemyBase.BP_EnemyBase_C|GetTargetPlayer _asbp_enemy_base)
            (:Is%20Valid
              (Game|SpawnActorfromClass "/Game/Blueprints/Projectiles/BP_EnemyProjectile.BP_EnemyProjectile_C" (Math|Transform|MakeTransform (Transformation|GetSocketLocation (Variables|/Script/Engine.Character|GetMesh _asbp_enemy_base) "Muzzle_Front") (Math|Rotator|FindLookatRotation (Transformation|GetSocketLocation (Variables|/Script/Engine.Character|GetMesh _asbp_enemy_base) "Muzzle_Front") (Transformation|GetActorLocation (Variables|/Game/Blueprints/Characters/Enemies/BP_EnemyBase.BP_EnemyBase_C|GetTargetPlayer _asbp_enemy_base))) "1.000000,1.000000,1.000000") "Undefined" "MultiplyWithRoot" 0 (Ability|MakeOutgoingGameplayEffectSpec "/Game/GameplayAbilitySystem/Enemies/Effects/GE_MinionDamage.GE_MinionDamage_C") 0))))))
    (:then_1
      (|PlayMontageandWaitProxy "None" "/Game/Blueprints/Characters/Enemies/Anims/AM_RangedAttack.AM_RangedAttack" 1.0 "None" true 1.0 0.0 false
        (:OnCompleted
          _)
        (:OnInterrupted
          _)
        (:OnCancelled
          _))
      (Ability|EndAbility))))

(event Ability|EventOnEndAbility
  (params (bWasCancelled :type Boolean)))