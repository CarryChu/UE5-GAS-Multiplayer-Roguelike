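; Lobby player controller that creates the lobby UI for the local player and reports their info to BP_LobbyGameMode.
; ROS (run-on-server) events toggle ready status, set the selected character class and request player info updates from the game mode.
; The character class's OnRep also triggers that game mode update.
; On match start, it shows the UI's loading screen and disables input.
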(event Custom|Updata%20Player%20Info
  (Utilities|FlowControl|Delay 0.1)
  (CallFunction|ROSUpdataPlayerInfo))

(event Custom|ROS_UpdataPlayerInfo
  (bind _asbp_lobby_game_mode (Utilities|Casting|CastToBP_LobbyGameMode (Game|GetGameMode)))
  (Default|UpdataPlayerInfo _asbp_lobby_game_mode self))

(event Custom|ROS_ToggleReadyStatus
  (bind _player_info (Variables|Default|GetPlayer%20Info))
  (Utilities|Struct|SetmembersinS_PlayerInfo _player_info (not (.Ready? (Utilities|Struct|BreakS_PlayerInfo _player_info))))
  (bind _asbp_lobby_game_mode (Utilities|Casting|CastToBP_LobbyGameMode (Game|GetGameMode)))
  (Default|UpdataPlayerInfo _asbp_lobby_game_mode self))

(event Custom|ROS_Updata%20Selected%20Character
  (params (Selected%20Character%20Class :type BP%20Third%20Person%20Character%20Class%20Reference))
  (Variables|Default|SetSelected%20Character%20Class Selected%20Character%20Class))

(event Custom|OnStartMatch
  (Default|ShowLoadingScreen (Variables|Default|GetLobby%20UI))
  (Input|DisableInput self))

(event EventBeginPlay
  (if (Pawn|IsLocalPlayerController)
    (bind _returnvalue (UserInterface|CreateWidget "/Game/Blueprints/UI/WBP_LobbyUI.WBP_LobbyUI_C"))
    (bind _output_get (Variables|Default|SetLobby%20UI _returnvalue))
    (UserInterface|Viewport|AddtoViewport _output_get 0)
    (Variables|Default|SetbShowMouseCursor true)
    (Input|SetInputModeGameandUI self (Variables|Default|GetLobby%20UI) "DoNotLock" true false)
    (CallFunction|ROSUpdataPlayerInfo)))

(fn ConstructionScript)

(fn OnRepSelectedCharacterClass
  (bind _asbp_lobby_game_mode (Utilities|Casting|CastToBP_LobbyGameMode (Game|GetGameMode)))
  (Default|UpdataPlayerInfo _asbp_lobby_game_mode self))