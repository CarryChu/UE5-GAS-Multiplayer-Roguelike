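; Eclipse gameplay ability that fires BP_Fireball projectiles from the Mage's muzzle, scaled by the player's Skill_Fireball card level.
; Six levels progress from one orb to yaw-offset spreads and a nine-orb curving ring that stops at end, with hit effects upgrading from Slow to GravityTear.
; A helper spawns each orb with a damage spec and a lifespan derived from an ability-system attribute divided by speed.
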(event Ability|EventActivateAbility
  (bind _lv6speed (Variables|Default|GetLv6Speed))
  (bind _lv5speed (Variables|Default|GetLv5Speed))
  (bind _lv4speed (Variables|Default|GetLv4Speed))
  ;[0.15 0.15 0.15 0.5] 法球生成
  (Ability|CommitAbility)
  (switch int (.Value (Utilities|Map|Find (Variables|/Script/MPRoguelike.UpgradeManagerComponent|GetOwnedCards (Variables|/Game/Blueprints/Characters/BP_CharacterPlayer.BP_CharacterPlayer_C|GetUpgradeManager (.AsBP%20Character%20Player (Utilities|Casting|CastToBP_CharacterPlayer (Ability|GetAvatarActorfromActorInfo))))) "Skill_Fireball"))
    (:1
      ;[0.15 0.15 0.15 0.5] Lv.1
      (CallFunction|SpawnEclipseFireball 0.0 0 1.0 1.0 0.0 false)
      (Ability|EndAbility))
    (:2
      ;[0.15 0.15 0.15 0.5] Lv.2
      (CallFunction|SpawnEclipseFireball 0.0 "/Game/GameplayAbilitySystem/Effects/GE_Eclipse_Slow.GE_Eclipse_Slow_C" 1.0 1.0 0.0 false)
      (Ability|EndAbility))
    (:3
      ;[0.15 0.15 0.15 0.5] Lv.3
      (CallFunction|SpawnEclipseFireball 0.0 "/Game/GameplayAbilitySystem/Effects/GE_Eclipse_Slow.GE_Eclipse_Slow_C" 1.0 1.0 0.0 false)
      (CallFunction|SpawnEclipseFireball 15.0 "/Game/GameplayAbilitySystem/Effects/GE_Eclipse_Slow.GE_Eclipse_Slow_C" 1.0 1.0 0.0 false)
      (CallFunction|SpawnEclipseFireball -15.0 "/Game/GameplayAbilitySystem/Effects/GE_Eclipse_Slow.GE_Eclipse_Slow_C" 1.0 1.0 0.0 false)
      (Ability|EndAbility))
    (:4
      ;[0.15 0.15 0.15 0.5] Lv.4
      (CallFunction|SpawnEclipseFireball 0.0 "/Game/GameplayAbilitySystem/Effects/GE_Eclipse_GravityTear.GE_Eclipse_GravityTear_C" 1.5 _lv4speed 0.0 false)
      (CallFunction|SpawnEclipseFireball 3e+01 "/Game/GameplayAbilitySystem/Effects/GE_Eclipse_GravityTear.GE_Eclipse_GravityTear_C" 1.5 _lv4speed 0.0 false)
      (CallFunction|SpawnEclipseFireball -3e+01 "/Game/GameplayAbilitySystem/Effects/GE_Eclipse_GravityTear.GE_Eclipse_GravityTear_C" 1.5 _lv4speed 0.0 false)
      (Ability|EndAbility))
    (:5
      ;[0.15 0.15 0.15 0.5] Lv.5
      (CallFunction|SpawnEclipseFireball 0.0 "/Game/GameplayAbilitySystem/Effects/GE_Eclipse_GravityTear.GE_Eclipse_GravityTear_C" 1.5 _lv5speed 0.0 false)
      (CallFunction|SpawnEclipseFireball 3e+01 "/Game/GameplayAbilitySystem/Effects/GE_Eclipse_GravityTear.GE_Eclipse_GravityTear_C" 1.5 _lv5speed 0.0 false)
      (CallFunction|SpawnEclipseFireball -3e+01 "/Game/GameplayAbilitySystem/Effects/GE_Eclipse_GravityTear.GE_Eclipse_GravityTear_C" 1.5 _lv5speed 0.0 false)
      (CallFunction|SpawnEclipseFireball 6e+01 "/Game/GameplayAbilitySystem/Effects/GE_Eclipse_GravityTear.GE_Eclipse_GravityTear_C" 1.5 _lv5speed 0.0 false)
      (CallFunction|SpawnEclipseFireball -6e+01 "/Game/GameplayAbilitySystem/Effects/GE_Eclipse_GravityTear.GE_Eclipse_GravityTear_C" 1.5 _lv5speed 0.0 false)
      (Ability|EndAbility))
    (:6
      ;[0.15 0.15 0.15 0.5] Lv.6
      (CallFunction|SpawnEclipseFireball 0.0 "/Game/GameplayAbilitySystem/Effects/GE_Eclipse_GravityTear.GE_Eclipse_GravityTear_C" 1.5 _lv6speed 1.2e+02 true)
      (CallFunction|SpawnEclipseFireball 4e+01 "/Game/GameplayAbilitySystem/Effects/GE_Eclipse_GravityTear.GE_Eclipse_GravityTear_C" 1.5 _lv6speed 1.2e+02 true)
      (CallFunction|SpawnEclipseFireball 8e+01 "/Game/GameplayAbilitySystem/Effects/GE_Eclipse_GravityTear.GE_Eclipse_GravityTear_C" 1.5 _lv6speed 1.2e+02 true)
      (CallFunction|SpawnEclipseFireball 1.2e+02 "/Game/GameplayAbilitySystem/Effects/GE_Eclipse_GravityTear.GE_Eclipse_GravityTear_C" 1.5 _lv6speed 1.2e+02 true)
      (CallFunction|SpawnEclipseFireball 1.6e+02 "/Game/GameplayAbilitySystem/Effects/GE_Eclipse_GravityTear.GE_Eclipse_GravityTear_C" 1.5 _lv6speed 1.2e+02 true)
      (CallFunction|SpawnEclipseFireball 2e+02 "/Game/GameplayAbilitySystem/Effects/GE_Eclipse_GravityTear.GE_Eclipse_GravityTear_C" 1.5 _lv6speed 1.2e+02 true)
      (CallFunction|SpawnEclipseFireball 2.4e+02 "/Game/GameplayAbilitySystem/Effects/GE_Eclipse_GravityTear.GE_Eclipse_GravityTear_C" 1.5 _lv6speed 1.2e+02 true)
      (CallFunction|SpawnEclipseFireball 2.8e+02 "/Game/GameplayAbilitySystem/Effects/GE_Eclipse_GravityTear.GE_Eclipse_GravityTear_C" 1.5 _lv6speed 1.2e+02 true)
      (CallFunction|SpawnEclipseFireball 3.2e+02 "/Game/GameplayAbilitySystem/Effects/GE_Eclipse_GravityTear.GE_Eclipse_GravityTear_C" 1.5 _lv6speed 1.2e+02 true)
      (Ability|EndAbility))))

(event Ability|EventOnEndAbility
  (params (bWasCancelled :type Boolean)))

(fn SpawnEclipseFireball
  (params (YawAngleOffset :type Float%20%28double-precision%29) (HitEffect :type Gameplay%20Effect%20Class%20Reference) (Size :type Float%20%28double-precision%29) (Speed :type Float%20%28double-precision%29) (CurveSpeed :type Float%20%28double-precision%29) (bStopAtEnd :type Boolean))
  (bind _returnvalue (Ability|GetAvatarActorfromActorInfo))
  (bind _returnvalue_2 (Ability|GetAbilitySystemComponent _returnvalue))
  (bind _asbp_mage (Utilities|Casting|CastToBP_Mage _returnvalue))
  (bind _muzzle (Variables|/Game/Blueprints/Characters/Player/BP_Mage.BP_Mage_C|GetMuzzle _asbp_mage))
  (bind _returnvalue_3 (Transformation|GetWorldTransform _muzzle))
  (bind (_location _rotation _scale) (Math|Transform|BreakTransform _returnvalue_3))
  (Game|SpawnActorfromClass "/Game/Blueprints/Projectiles/BP_Fireball.BP_Fireball_C" (Math|Transform|MakeTransform _location (Math|Rotator|CombineRotators _rotation (Math|Rotator|MakeRotator 0.0 0.0 YawAngleOffset)) _scale) "Undefined" "MultiplyWithRoot" 0 (/ (.ReturnValue (Ability|Attribute|GetFloatAttributefromAbilitySystemComponent _returnvalue_2 "(AttributeName=\"AttackRange\",Attribute=/Script/MPRoguelike.BasicAttributeSet:AttackRange,AttributeOwner=\"/Script/CoreUObject.Class'/Script/MPRoguelike.BasicAttributeSet'\")")) (* 1.5e+03 Speed)) (GameplayEffects|MakeOutgoingSpec :self _returnvalue_2 :GameplayEffectClass "/Game/GameplayAbilitySystem/Effects/GE_FireballDamage.GE_FireballDamage_C") HitEffect Size Speed CurveSpeed bStopAtEnd 0)
  (return))